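; Teleporter actor that moves any actor overlapping its sphere to a destination marked by an Arrow component.
; The construction script places the Arrow using the TeleportLocation transform.
; On sphere overlap, the actor's root takes the Arrow's world location and rotation.
; For the player character, it also aligns the controller's rotation to the new facing and zeroes movement velocity.
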(event `self.Sphere.OnComponentBeginOverlap`
  (params (OverlappedComponent :type "PrimitiveComponent Object Reference") (OtherActor :type "Actor Object Reference") (OtherComp :type "PrimitiveComponent Object Reference") (OtherBodyIndex :type Integer) (bFromSweep :type Boolean) (SweepResult :type "HitResult Structure (by ref)"))
  (bind _returnvalue (`GameplayStatics.GetPlayerCharacter` 0))
  (bind (_returnvalue_location _returnvalue_rotation) (`KismetMathLibrary.BreakTransform` (`SceneComponent.K2_GetComponentToWorld` (`self.Arrow`))))
  (`SceneComponent.K2_SetWorldTransform` (`Actor.RootComponent` OtherActor) (`KismetMathLibrary.MakeTransform` _returnvalue_location _returnvalue_rotation) false false)
  (if (== OtherActor _returnvalue)
    (`Controller.SetControlRotation` (`GameplayStatics.GetPlayerController` 0) (`self.K2_GetActorRotation` _returnvalue))
    (set `MovementComponent.Velocity` (0.0 0.0 0.0) (`Character.CharacterMovement` _returnvalue))))

(fn `UserConstructionScript`
  (`SceneComponent.K2_SetRelativeTransform` (`self.Arrow`) (`self.Teleport Location`) false false))