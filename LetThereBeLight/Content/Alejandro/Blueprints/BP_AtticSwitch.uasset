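; BP_AtticSwitch is a light switch that the player works with the E key while inside its box trigger.
; On BeginPlay it caches every BP_Light in the level into LightArray.
; Box overlap enables input and opens a gate; leaving reverses both.
; A gated E press calls ToggleLightsMessage on each cached light whose LightIndex matches the switch's, while an older LightHolder visibility toggle remains unconnected.
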(event `self.ReceiveBeginPlay`
  (bind _outactors (`GameplayStatics.GetAllActorsOfClass` "/Game/Alejandro/Blueprints/BP_Light.BP_Light_C"))
  (for _array_element _outactors
    (`KismetArrayLibrary.Array_Add` (`self.Light Array`) _array_element)))

(event `Key|E`
  (params (Key :type "Key Structure"))
  (:`Pressed`
    (`/Engine/EditorBlueprintResources/StandardMacros.Gate` true :!label _label
      (:`Exit`
        (for _array_element (`self.Light Array`)
          (if (== (`/Game/Alejandro/Blueprints/BP_Light.Light Index` _array_element) (`self.Light Index`))
            (message `/Game/Alejandro/Blueprints/LightsInterface.ToggleLights` _array_element)))))))

(event `self.Box.OnComponentBeginOverlap`
  (params (OverlappedComponent :type "PrimitiveComponent Object Reference") (OtherActor :type "Actor Object Reference") (OtherComp :type "PrimitiveComponent Object Reference") (OtherBodyIndex :type Integer) (bFromSweep :type Boolean) (SweepResult :type "HitResult Structure (by ref)"))
  (`self.EnableInput` (`GameplayStatics.GetPlayerController` 0))
  (goto _label :!via `Open`))

(event `self.Box.OnComponentEndOverlap`
  (params (OverlappedComponent :type "PrimitiveComponent Object Reference") (OtherActor :type "Actor Object Reference") (OtherComp :type "PrimitiveComponent Object Reference") (OtherBodyIndex :type Integer))
  (`self.DisableInput` (`GameplayStatics.GetPlayerController` 0))
  (goto _label :!via `Close`))

(fn `UserConstructionScript`)