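; BP_Key is a key pickup that the player collects by pressing Interact while standing near it.
; Overlap of its Box with BPNYC_Character caches the character, enables input on the actor and opens a Gate, while end overlap reverses the input and Gate changes.
; A press through the open Gate sets HasKey on the character, plays a pickup sound and destroys the key.
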(event `InputAction|Interact`
  (params (Key :type "Key Structure"))
  (:`Pressed`
    (`/Engine/EditorBlueprintResources/StandardMacros.Gate` true :!label _label
      (:`Exit`
        (set `/Game/Alejandro/Blueprints/BPNYC_Character.HasKey?` true (stale `self.Box.OnComponentBeginOverlap` _asbpnyc_character))
        (`GameplayStatics.PlaySoundAtLocation` "/Engine/VREditor/Sounds/UI/Object_PickUp.Object_PickUp" (`self.K2_GetActorLocation`) (struct) 1.0 1.0 0.0 null null null null)
        (`self.K2_DestroyActor`)))))

(event `self.Box.OnComponentBeginOverlap`
  (params (OverlappedComponent :type "PrimitiveComponent Object Reference") (OtherActor :type "Actor Object Reference") (OtherComp :type "PrimitiveComponent Object Reference") (OtherBodyIndex :type Integer) (bFromSweep :type Boolean) (SweepResult :type "HitResult Structure (by ref)"))
  (bind _asbpnyc_character (cast `/Game/Alejandro/Blueprints/BPNYC_Character` OtherActor))
  (`self.EnableInput` (`GameplayStatics.GetPlayerController` 0))
  (goto _label :!via `Open`))

(event `self.Box.OnComponentEndOverlap`
  (params (OverlappedComponent :type "PrimitiveComponent Object Reference") (OtherActor :type "Actor Object Reference") (OtherComp :type "PrimitiveComponent Object Reference") (OtherBodyIndex :type Integer))
  (cast `/Game/Alejandro/Blueprints/BPNYC_Character` OtherActor)
  (`self.DisableInput` (`GameplayStatics.GetPlayerController` 0))
  (goto _label :!via `Close`))

(fn `UserConstructionScript`)