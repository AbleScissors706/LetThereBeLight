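; TrashcanHole_BP is a trash can opening that detects thrown pizza boxes and counts them as trashed pizza.
; Its Box overlap event accepts only actors of exact class BP_PizzaBoxThrown and destroys them.
; It then plays a random BoxSound entry at its location with randomized volume and increments TrashedPizza on the player's BPNYC_Character.
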(event `self.Box.OnComponentBeginOverlap`
  (params (OverlappedComponent :type "PrimitiveComponent Object Reference") (OtherActor :type "Actor Object Reference") (OtherComp :type "PrimitiveComponent Object Reference") (OtherBodyIndex :type Integer) (bFromSweep :type Boolean) (SweepResult :type "HitResult Structure (by ref)"))
  (if (== (`GameplayStatics.GetObjectClass` OtherActor) "/Game/WhiteboxMeshFolder/BP_PizzaBoxThrown.BP_PizzaBoxThrown_C")
    (`self.K2_DestroyActor` OtherActor)
    (`GameplayStatics.PlaySoundAtLocation` (`KismetArrayLibrary.Array_Random` (`self.BoxSound`)) (`self.K2_GetActorLocation`) (struct) (`KismetMathLibrary.RandomFloatInRange` 1.5 2.5) 1.0 0.0 "/Game/Audio/nycsounds/Attenuation.Attenuation" null null null)
    (bind _asbpnyc_character (cast `/Game/ThirdPerson/Alejandro/Blueprints/BPNYC_Character` (`GameplayStatics.GetPlayerPawn` 0)))
    (set `/Game/ThirdPerson/Alejandro/Blueprints/BPNYC_Character.TrashedPizza` (+ (`/Game/ThirdPerson/Alejandro/Blueprints/BPNYC_Character.TrashedPizza` _asbpnyc_character) 1) _asbpnyc_character)))

(fn `UserConstructionScript`)